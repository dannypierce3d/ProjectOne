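; Teleporter actor that moves the player between screens, switching to a new camera and placing the pawn at a target actor facing a set direction.
; On overlap it disables player actions via game instance flags, fades to white, teleports, then fades back in.
; An IsTeleporting flag stops the arrival from retriggering a teleport.
; Tick then forces a short step forward before re-enabling movement, jumping and slashing.
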(event EventTick
  (params (DeltaSeconds :type Float%20%28single-precision%29))
  (bind _upordown (Variables|Default|GetupOrDown))
  (bind _leftorright (Variables|Default|GetleftOrRight))
  (bind _returnvalue (Math|Vector|MakeVector _upordown _leftorright 0.0))
  ;[1 1 1] Walk Up
  (if (not (Variables|Default|GetstepForward)) ; Checks to see if character teleported to make him step forward
    (Transformation|SetActorRotation (Game|GetPlayerCharacter 0) (Math|Conversions|RotationFromXVector _returnvalue))
    (bind _asbp_game_instance (Utilities|Casting|CastToBP_GameInstance (Game|GetGameInstance)))
    (Variables|/Game/Blueprints/BP_GameInstance.BP_GameInstance_C|SetisBlocking? _asbp_game_instance false)
    (Pawn|Input|AddMovementInput (Game|GetPlayerCharacter 0) _returnvalue 1.0 true)
    (bind _asbp_game_instance_2 (Utilities|Casting|CastToBP_GameInstance (Game|GetGameInstance)))
    (Variables|/Game/Blueprints/BP_GameInstance.BP_GameInstance_C|SetisTransferingScreen? _asbp_game_instance_2 true)
    (Utilities|FlowControl|Delay 0.3)
    (Variables|Default|SetstepForward true)
    (bind _asbp_game_instance_3 (Utilities|Casting|CastToBP_GameInstance (Game|GetGameInstance)))
    (Variables|/Game/Blueprints/BP_GameInstance.BP_GameInstance_C|SetallowMovement? _asbp_game_instance_3 true)
    (bind _asbp_game_instance_4 (Utilities|Casting|CastToBP_GameInstance (Game|GetGameInstance)))
    (Variables|/Game/Blueprints/BP_GameInstance.BP_GameInstance_C|SetallowJumping? _asbp_game_instance_4 true)
    (bind _asbp_game_instance_5 (Utilities|Casting|CastToBP_GameInstance (Game|GetGameInstance)))
    (Variables|/Game/Blueprints/BP_GameInstance.BP_GameInstance_C|SetallowSlashing? _asbp_game_instance_5 true)))

(event EventActorBeginOverlap
  (params (OtherActor :type Actor%20Object%20Reference))
  (bind _teleportto (Variables|Default|GetteleportTo))
  (bind _returnvalue (Transformation|GetActorLocation _teleportto))
  (bind (_x _y _z) (Math|Vector|BreakVector _returnvalue))
  ;[1 1 1] Teleport
  (bind _asbp_game_instance (Utilities|Casting|CastToBP_GameInstance (Game|GetGameInstance)))
  (Variables|/Game/Blueprints/BP_GameInstance.BP_GameInstance_C|SetallowJumping? _asbp_game_instance false)
  (bind _asbp_game_instance_2 (Utilities|Casting|CastToBP_GameInstance (Game|GetGameInstance)))
  (Variables|/Game/Blueprints/BP_GameInstance.BP_GameInstance_C|SetallowSlashing? _asbp_game_instance_2 false)
  (bind _asbp_game_instance_3 (Utilities|Casting|CastToBP_GameInstance (Game|GetGameInstance)))
  (if (Variables|/Game/Blueprints/BP_GameInstance.BP_GameInstance_C|GetisTeleporting? _asbp_game_instance_3)
    (Utilities|FlowControl|Delay 1.0)
    (bind _asbp_game_instance_4 (Utilities|Casting|CastToBP_GameInstance (Game|GetGameInstance)))
    (Variables|/Game/Blueprints/BP_GameInstance.BP_GameInstance_C|SetisTeleporting? _asbp_game_instance_4 false)
    (else
      (CameraFades|StartCameraFade (Game|GetPlayerCameraManager 0) 0.0 1.0 0.35 "(R=1.000000,G=1.000000,B=1.000000,A=1.000000)" false false)
      (bind _asbp_game_instance_5 (Utilities|Casting|CastToBP_GameInstance (Game|GetGameInstance)))
      (Variables|/Game/Blueprints/BP_GameInstance.BP_GameInstance_C|SetisTeleporting? _asbp_game_instance_5 true)
      (bind _asbp_game_instance_6 (Utilities|Casting|CastToBP_GameInstance (Game|GetGameInstance)))
      (Variables|/Game/Blueprints/BP_GameInstance.BP_GameInstance_C|SetallowMovement? _asbp_game_instance_6 false)
      (Utilities|FlowControl|Delay 0.35)
      (Game|Player|SetViewTargetwithBlend (Game|GetPlayerController 0) (Variables|Default|GetnewCamera) 0.0 "VTBlend_EaseIn" 0.0 true)
      (Transformation|Teleport (Game|Player|GetPlayerPawn 0) (Math|Vector|MakeVector (+ _x 0.0) _y _z) (Math|Conversions|RotationFromXVector (Math|Vector|MakeVector (Variables|Default|GetupOrDown) (Variables|Default|GetleftOrRight) 0.0)))
      (CameraFades|StartCameraFade (Game|GetPlayerCameraManager 0) 1.0 0.0 0.35 "(R=1.000000,G=1.000000,B=1.000000,A=1.000000)" false false)
      (Variables|Default|SetstepForward false)
      (Utilities|FlowControl|Delay 1.0)
      (bind _asbp_game_instance_7 (Utilities|Casting|CastToBP_GameInstance (Game|GetGameInstance)))
      (Variables|/Game/Blueprints/BP_GameInstance.BP_GameInstance_C|SetisTeleporting? _asbp_game_instance_7 false))))

(fn ConstructionScript)