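; BP_ArrowFlash_01 is an arrow flash actor, apparently meant to travel along the player's bow and then spin.
; MoveToTip nudges the Scene component along local X with a debug print, and Spin rotates it in small steps.
; The sequence that attaches it to the character's BowTest01 and drives both events with looping timers is disconnected, so nothing in this file starts the motion.
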(event Custom|MoveToTip
  (Development|PrintString "Hello")
  (Transformation|AddRelativeLocation (Variables|Default|GetScene) "0.150000, 0, 0" false false))

(event Custom|Spin
  (Transformation|AddLocalRotation (Variables|Default|GetScene) "0, 0,3.000000" false false))

(event Collision|EventActorBeginOverlap
  (params (OtherActor :type Actor%20Object%20Reference)))

(event EventTick
  (params (DeltaSeconds :type Float%20%28single-precision%29)))

(event EventBeginPlay)

(fn ConstructionScript)