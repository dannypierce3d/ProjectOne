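; BP_Spike_01 is a spike hazard that damages and knocks back the player character.
; Box overlaps with a BP_Character set or clear a flag, and entry starts a Delay-driven polling loop that repeats while it is set.
; When player 0 is not invincible, the loop triggers invincibility, launches them against their horizontal movement with a strong downward force, and applies damage.
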(event OnComponentBeginOverlap(Box)
  (params (OverlappedComponent :type Primitive%20Component%20Object%20Reference) (OtherActor :type Actor%20Object%20Reference) (OtherComp :type Primitive%20Component%20Object%20Reference) (OtherBodyIndex :type Integer) (bFromSweep :type Boolean) (SweepResult :type Hit%20Result%20Structure%20%28by%20ref%29))
  ;[1 1 1] Is standing on spikes
  (Utilities|Casting|CastToBP_Character OtherActor)
  (Variables|Default|SetisOnSpikes true)
  (CallFunction|StandingonSpikes))

(event OnComponentEndOverlap(Box)
  (params (OverlappedComponent :type Primitive%20Component%20Object%20Reference) (OtherActor :type Actor%20Object%20Reference) (OtherComp :type Primitive%20Component%20Object%20Reference) (OtherBodyIndex :type Integer))
  ;[1 1 1] Is not standing on spikes
  (Utilities|Casting|CastToBP_Character OtherActor)
  (Variables|Default|SetisOnSpikes false))

(event Custom|StandingOnSpikes
  (bind _returnvalue (Game|GetPlayerCharacter 0))
  ;[1 1 1] Knockback character and decrease health
  (if (Variables|Default|GetisOnSpikes) :!label _label
    (bind _asbp_character (Utilities|Casting|CastToBP_Character (Game|GetPlayerCharacter 0)))
    (if (Variables|/Game/Blueprints/PlayerCharacter/BP_Character.BP_Character_C|GetisInvincible? _asbp_character)
      _
      (else
        (Default|Invincible _asbp_character)
        (Character|LaunchCharacter _returnvalue (Math|Vector|MakeVector (.x (* (Math|Vector|MakeVector (.x (Math|Vector|Normalize (Transformation|GetVelocity _asbp_character))) (.y (Math|Vector|Normalize (Transformation|GetVelocity _asbp_character))) 0.0) -1.2e+03)) (.y (* (Math|Vector|MakeVector (.x (Math|Vector|Normalize (Transformation|GetVelocity _asbp_character))) (.y (Math|Vector|Normalize (Transformation|GetVelocity _asbp_character))) 0.0) -1.2e+03)) -3e+03) true true)
        (bind _asbp_character_2 (Utilities|Casting|CastToBP_Character _returnvalue))
        (Default|TakeDamage _asbp_character_2 0.5)))
    (Utilities|FlowControl|Delay 0.2)
    (goto _label)))

(fn ConstructionScript)