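; BP_ArrowDisplay_01 is the cosmetic arrow shown on the player's bow while a shot is charging.
; On BeginPlay it attaches to the character's bow and runs a looping timer for two seconds that nudges its Sphere forward as a charge animation.
; Tick snaps it to the launch point with the bow's rotation, yaw flipped 180 degrees, and destroys it once charging stops.
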(event Custom|MoveToTip
  ;[1 1 1] Charging animation
  (Transformation|AddRelativeLocation (Variables|Default|GetSphere) "0.150000,0.000000, 0" false false))

(event EventBeginPlay
  ;[1 1 1] Attach display arrow to character bow and start charging animation
  (bind _asbp_character (Utilities|Casting|CastToBP_Character (Game|GetPlayerCharacter 0)))
  (Transformation|AttachComponentToComponent (Variables|/Game/Blueprints/BP_Character.BP_Character_C|GetBowTest_01 _asbp_character) "None" "KeepRelative" "SnapToTarget" "KeepWorld" false)
  (Utilities|Time|SetTimerbyFunctionName 0 "MoveToTip" 0.005 true)
  (Utilities|FlowControl|Delay 2.0)
  (Utilities|Time|ClearTimerbyFunctionName 0 "MoveToTip"))

(event EventTick
  (params (DeltaSeconds :type Float%20%28single-precision%29))
  ;[1 1 1] Destroy display arrow if not charging
  (bind _asbp_character (Utilities|Casting|CastToBP_Character (Game|GetPlayerCharacter 0)))
  (if (Variables|/Game/Blueprints/BP_Character.BP_Character_C|GetisCharging? _asbp_character)
    (bind _asbp_character_2 (Utilities|Casting|CastToBP_Character (Game|GetPlayerCharacter 0)))
    (Transformation|SetActorLocation (Transformation|GetWorldLocation (Variables|/Game/Blueprints/BP_Character.BP_Character_C|GetArrowLaunchPoint _asbp_character_2)) false false)
    (Transformation|SetActorRotation (Math|Rotator|MakeRotator (.roll (Transformation|GetWorldRotation (Variables|/Game/Blueprints/BP_Character.BP_Character_C|GetBowTest_01 _asbp_character_2))) (.pitch (Transformation|GetWorldRotation (Variables|/Game/Blueprints/BP_Character.BP_Character_C|GetBowTest_01 _asbp_character_2))) (+ (.yaw (Transformation|GetWorldRotation (Variables|/Game/Blueprints/BP_Character.BP_Character_C|GetBowTest_01 _asbp_character_2))) 1.8e+02)))
    (else
      (Actor|DestroyActor))))

(fn ConstructionScript)