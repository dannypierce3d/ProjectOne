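; BP_HeartPiece_01 is a heart pickup that permanently raises the player character's maximum health.
; On the first actor overlap, guarded by a DoOnce, it adds one to BP_Character's MaxHealth, capped at a limit, and refills Health to the new maximum.
; The overlapping actor is not checked; the player character is fetched directly.
; It then hides itself and destroys itself after a short delay.
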(event EventBeginPlay)

(event Collision|EventActorBeginOverlap
  (params (OtherActor :type Actor%20Object%20Reference))
  (Utilities|FlowControl|DoOnce false
    (:Completed
      (bind _asbp_character (Utilities|Casting|CastToBP_Character (Game|GetPlayerCharacter 0)))
      (bind _output_get (Variables|/Game/Blueprints/BP_Character.BP_Character_C|SetmaxHealth _asbp_character (Math|Float|Clamp(Float) (+ (Variables|/Game/Blueprints/BP_Character.BP_Character_C|GetmaxHealth _asbp_character) 1.0) 0.0 14.0)))
      (Variables|/Game/Blueprints/BP_Character.BP_Character_C|Sethealth _asbp_character _output_get)
      (Rendering|SetActorHiddenInGame true)
      (Utilities|FlowControl|Delay 3.0)
      (Actor|DestroyActor))))

(event EventTick
  (params (DeltaSeconds :type Float%20%28single-precision%29)))

(fn ConstructionScript)