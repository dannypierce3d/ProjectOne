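; BP_Inventory is a slot-based inventory that sizes its Slots array on BeginPlay and stores an item class and amount per slot.
; AddItem tops up partial stacks or claims empty slots via the search helpers, recursing for overflow and extra non-stackable items while ignoring the recursive result.
; Query functions report slot contents, but GetItemInfoAtIndex, stack top-ups and non-stackable adds use slot 0 instead of the requested or found index.
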(event EventBeginPlay
  (Utilities|Array|Resize (Variables|Default|GetSlots) (Variables|Default|GetAmountOfSlots)))

(event Collision|EventActorBeginOverlap
  (params (OtherActor :type Actor%20Object%20Reference)))

(event EventTick
  (params (DeltaSeconds :type Float%20%28single-precision%29)))

(fn ConstructionScript)

(fn IsSlotEmpty?
  (params (Index :type Integer))
  (return (not (Utilities|IsValidClass (.ItemClass (Utilities|Struct|BreakS_InventorySlot (Utilities|Array|Get(acopy) (Variables|Default|GetSlots) Index)))))))

(fn GetItemInfoatIndex
  (params (Index :type Integer))
  (bind _slots (Variables|Default|GetSlots))
  (bind _output (Utilities|Array|Get(acopy) _slots))
  (bind (_itemclass _amount) (Utilities|Struct|BreakS_InventorySlot _output))
  (if (Utilities|IsValidClass _itemclass)
    (return false (Utilities|GetClassDefaults _itemclass) _amount) ; Valid
    (else
      (return true "" 0) ; Not valid
    )))

(fn SearchEmptySlot
  (bind (_array_element _array_index) (Utilities|Array|ForEachLoopwithBreak (Variables|Default|GetSlots) :!label _label) ; Run through slots array to find first empty slot
    (:LoopBody
      (if (not (Utilities|IsValidClass (.ItemClass (Utilities|Struct|BreakS_InventorySlot _array_element))))
        (LocalVariables|SetlocalBool true) ; Return Success if empty slot found
        (LocalVariables|SetlocalIndex _array_index) ; Index where empty slot was found
        (goto _label Break)))
    (:Completed
      (return (LocalVariables|GetlocalBool) (LocalVariables|GetlocalIndex)))))

(fn SearchFreeStack
  (params (ItemClass :type BP%20Master%20Item%20Class%20Reference))
  (bind (_array_element _array_index) (Utilities|Array|ForEachLoopwithBreak (Variables|Default|GetSlots) :!label _label)
    (:LoopBody
      (if (Utilities|IsValidClass (.ItemClass (Utilities|Struct|BreakS_InventorySlot _array_element)))
        (if (and (== (.ItemClass (Utilities|Struct|BreakS_InventorySlot _array_element)) ItemClass) (< (.Amount (Utilities|Struct|BreakS_InventorySlot _array_element)) (Variables|Default|GetMaxStackSize)))
          (LocalVariables|SetlocalBool true) ; If item class is right and stack isn't full
          (LocalVariables|SetlocalIndex _array_index)
          (goto _label Break))))
    (:Completed
      (return (LocalVariables|GetlocalBool) (LocalVariables|GetlocalIndex)))))

(fn AddItem
  (params (ItemClass :type BP%20Master%20Item%20Class%20Reference) (Amount :type Integer))
  (LocalVariables|SetlocalClass ItemClass) ; Item type to add
  (LocalVariables|SetlocalAmount Amount) ; Amount of item to attempt to add
  (if (.canBeStacked? (Utilities|Struct|BreakS_ItemInfo (Utilities|GetClassDefaults ItemClass)))
    (bind _success_ (CallFunction|SearchFreeStack (LocalVariables|GetlocalClass))) ; Item class is stackable so search for free stack
    (if _success_
      (LocalVariables|SetFoundIndex 0) ; Found stack to add to
      (if (> (+ (.Amount (Utilities|Struct|BreakS_InventorySlot (Utilities|Array|Get(acopy) (Variables|Default|GetSlots) (LocalVariables|GetFoundIndex)))) (LocalVariables|GetlocalAmount)) (Variables|Default|GetMaxStackSize))
        (LocalVariables|SetlocalAmount (- (+ (.Amount (Utilities|Struct|BreakS_InventorySlot (Utilities|Array|Get(acopy) (Variables|Default|GetSlots) (LocalVariables|GetFoundIndex)))) (LocalVariables|GetlocalAmount)) (Variables|Default|GetMaxStackSize)))
        (Utilities|Array|SetArrayElem (Variables|Default|GetSlots) (LocalVariables|GetFoundIndex) (Utilities|Struct|MakeS_InventorySlot (LocalVariables|GetlocalClass) (Variables|Default|GetMaxStackSize))) ; Fill up stack then add remainder to new stack
        (CallFunction|AddItem (LocalVariables|GetlocalClass) (LocalVariables|GetlocalAmount)) ; Take remaining and add to new stack
        (return true 0)
        (else
          (Utilities|Array|SetArrayElem (Variables|Default|GetSlots) (LocalVariables|GetFoundIndex) (Utilities|Struct|MakeS_InventorySlot (LocalVariables|GetlocalClass) (+ (.Amount (Utilities|Struct|BreakS_InventorySlot (Utilities|Array|Get(acopy) (Variables|Default|GetSlots) (LocalVariables|GetFoundIndex)))) (LocalVariables|GetlocalAmount)))) ; Add amount to existing amount in stack
          (return true 0)))
      (else
        (bind (_success__2 _index) (CallFunction|SearchEmptySlot)) ; Could not find free stack so make new stack in next empty slot
        (if _success__2
          (bind _output_get (LocalVariables|SetFoundIndex _index)) ; Found empty index
          (if (> (LocalVariables|GetlocalAmount) (Variables|Default|GetMaxStackSize)) ; Check if amount is > Max Stack Size
            (Utilities|Array|SetArrayElem (Variables|Default|GetSlots) _output_get (Utilities|Struct|MakeS_InventorySlot (LocalVariables|GetlocalClass) (Variables|Default|GetMaxStackSize))) ; Fill stack
            (CallFunction|AddItem (LocalVariables|GetlocalClass) (- (LocalVariables|GetlocalAmount) (Variables|Default|GetMaxStackSize))) ; Add remaining stack
            (return true 0)
            (else
              (Utilities|Array|SetArrayElem (Variables|Default|GetSlots) (LocalVariables|GetFoundIndex) (Utilities|Struct|MakeS_InventorySlot (LocalVariables|GetlocalClass) (LocalVariables|GetlocalAmount))) ; Adds amount to free stack
              (return true 0)))
          (else
            (return false 0) ; Could not add item
          ))))
    (else
      (bind _success__3 (CallFunction|SearchEmptySlot)) ; Find first empty slot
      (if _success__3
        (bind _output_get_2 (LocalVariables|SetFoundIndex 0)) ; Index to use
        (Utilities|Array|SetArrayElem (Variables|Default|GetSlots) _output_get_2 (Utilities|Struct|MakeS_InventorySlot (LocalVariables|GetlocalClass) 1)) ; Only 1 for Item Amount as this cannot be stacked
        (if (> (LocalVariables|GetlocalAmount) 1) ; Check if more than one of item class needs to be added
          (CallFunction|AddItem (LocalVariables|GetlocalClass) (- (LocalVariables|GetlocalAmount) 1)) ; Adds remaining items
        )
        (return true 0)
        (else
          (return false (LocalVariables|GetlocalAmount)) ; Could not add item.
        )))))

(fn GetAmountatIndex
  (params (Index :type Integer))
  (return (.Amount (Utilities|Struct|BreakS_InventorySlot (Utilities|Array|Get(acopy) (Variables|Default|GetSlots) Index)))))