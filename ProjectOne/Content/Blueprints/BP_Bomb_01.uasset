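; Bomb actor that, when its fuse is lit at BeginPlay, flashes and explodes after a fixed delay.
; A timeline drives the flash on a dynamic material, then the actor spawns BP_BombExplosion_01 and destroys itself; DestroyBomb triggers this after a shorter delay.
; Tick adds downward acceleration while the box simulates physics for a faster fall.
; Leftover bush logic can spawn a ruby, but its hit and sword/arrow triggers are disconnected.
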(event OnComponentBeginOverlap(Bomb)
  (params (OverlappedComponent :type Primitive%20Component%20Object%20Reference) (OtherActor :type Actor%20Object%20Reference) (OtherComp :type Primitive%20Component%20Object%20Reference) (OtherBodyIndex :type Integer) (bFromSweep :type Boolean) (SweepResult :type Hit%20Result%20Structure%20%28by%20ref%29))
  ;[1 1 1] Destroy with sword only when attacking
)

(event OnComponentHit(Box)
  (params (HitComponent :type Primitive%20Component%20Object%20Reference) (OtherActor :type Actor%20Object%20Reference) (OtherComp :type Primitive%20Component%20Object%20Reference) (NormalImpulse :type Vector :default "0, 0, 0") (Hit :type Hit%20Result%20Structure%20%28by%20ref%29))
  ;[1 1 1] Destroy Bush when thrown/dropped
)

(event Custom|SpawnItem
  (bind _returnvalue (Transformation|GetActorTransform))
  ;[1 1 1] Spawn Item
  (Utilities|FlowControl|DoOnce false
    (:Completed
      (bind _returnvalue_2 (Game|SpawnActorfromClass "/Game/Blueprints/BP_Ruby_02.BP_Ruby_02_C" (Transformation|GetActorTransform) "AlwaysSpawn" 0 0))
      (bind _output_get (Variables|Default|SetSpawn_Ruby _returnvalue_2))
      (Transformation|SetActorTransform _output_get (Math|Transform|MakeTransform (.location _returnvalue) (.rotation _returnvalue) "1,1,1")))))

(event Custom|DestroyBush
  ;[1 1 1] Destroy Bush
  (Utilities|FlowControl|DoOnce false
    (:Completed
      (Rendering|SetActorHiddenInGame true)
      (Utilities|FlowControl|Delay 0.1)
      (CallFunction|SpawnItem)
      (Actor|DestroyActor))))

(event Custom|DestroyBomb
  (Utilities|FlowControl|Delay 0.15)
  (bind _output_get (Variables|Default|SetexplosionLocation (Transformation|GetActorLocation)))
  (Components|DestroyComponent (Variables|Default|GetBox))
  (Game|SpawnActorfromClass "/Game/Blueprints/BP_BombExplosion_01.BP_BombExplosion_01_C" (Math|Transform|MakeTransform _output_get "0, 0, 0" "1,1,1") "AlwaysSpawn" 0 0)
  (Actor|DestroyActor))

(event Custom|StartBombFlash
  (bind _newtrack_0 (Timeline|bombFlash PlayFromStart)
    (:Update
      (Rendering|Material|SetScalarParameterValue (Variables|Default|GetdynamicMaterial) "bombFlash" _newtrack_0 :!class /Script/Engine.MaterialInstanceDynamic))))

(event Custom|FallSpeed)

(event EventTick
  (params (DeltaSeconds :type Float%20%28single-precision%29))
  ;[1 1 1] Fall speed
  (if (Physics|IsSimulatingPhysics (Variables|Default|GetBox) "None")
    (Physics|AddForce (Variables|Default|GetBox) (Math|Vector|MakeVector 0.0 0.0 -5e+03) "None" true)))

(event EventBeginPlay
  (if (Variables|Default|GetisFuseLit?)
    (bind _returnvalue (Rendering|Material|CreateDynamicMaterialInstance "/Game/Materials/BombMaterial_Dynamic.BombMaterial_Dynamic" :!class /Script/Engine.KismetMaterialLibrary))
    (bind _output_get (Variables|Default|SetdynamicMaterial _returnvalue))
    (Rendering|Material|SetMaterial (Variables|Default|GetBomb) 0 _output_get)
    (CallFunction|StartBombFlash)
    (Utilities|FlowControl|Delay 4.0)
    (bind _output_get_2 (Variables|Default|SetexplosionLocation (Transformation|GetActorLocation)))
    (Components|DestroyComponent (Variables|Default|GetBox))
    (Game|SpawnActorfromClass "/Game/Blueprints/BP_BombExplosion_01.BP_BombExplosion_01_C" (Math|Transform|MakeTransform _output_get_2 "0, 0, 0" "1,1,1") "AlwaysSpawn" 0 0)
    (Actor|DestroyActor)))

(fn ConstructionScript)