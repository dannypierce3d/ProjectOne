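; Arrow projectile that gets an upward launch impulse on spawn and turns to face its velocity through a per-frame looping timer.
; Overlap with "arrowstick" components freezes it, blinks it via an opacity timeline on a dynamic material, then destroys it.
; Overlap with "arrowwilldestroy" actors destroys it only when IsChargedShot is false.
; Leaving an "arrowdestroy" volume disables physics and collision after a delay, then destroys it.
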(event OnComponentEndOverlap(Collision)
  (params (OverlappedComponent :type Primitive%20Component%20Object%20Reference) (OtherActor :type Actor%20Object%20Reference) (OtherComp :type Primitive%20Component%20Object%20Reference) (OtherBodyIndex :type Integer))
  (bind _collision (Variables|Default|GetCollision))
  ;[1 1 1] Destroy arrow if it leaves screen
  (if (Components|ComponentHasTag OtherComp "arrowdestroy")
    (Utilities|FlowControl|Delay 1.0)
    (Physics|SetSimulatePhysics _collision false)
    (Collision|SetCollisionEnabled _collision "NoCollision")
    (Utilities|FlowControl|Delay 1.0)
    (Development|PrintString "ARROWLEFTSCREEN")
    (Actor|DestroyActor)))

(event OnComponentBeginOverlap(Collision)
  (params (OverlappedComponent :type Primitive%20Component%20Object%20Reference) (OtherActor :type Actor%20Object%20Reference) (OtherComp :type Primitive%20Component%20Object%20Reference) (OtherBodyIndex :type Integer) (bFromSweep :type Boolean) (SweepResult :type Hit%20Result%20Structure%20%28by%20ref%29))
  ;[1 1 1] Find if arrow should destroy object or get stuck in object
  (if (Components|ComponentHasTag OtherComp "arrowstick")
    (Components|DestroyComponent (Variables|Default|GetProjectileMovement))
    (Class|KismetSystemLibrary|PauseTimer 0 "RotateTowardsVelocity")
    (Physics|SetSimulatePhysics (Variables|Default|GetCollision) false)
    (Utilities|FlowControl|Delay 0.5)
    (CallFunction|Blinking)
    (Utilities|FlowControl|Delay 0.5)
    (Actor|DestroyActor)
    (elif (Actor|ActorHasTag OtherActor "arrowwilldestroy")
      (if (not (Variables|Default|GetisChargedShot?))
        (Utilities|FlowControl|Delay 0.05)
        (Actor|DestroyActor)))))

(event Custom|RotateTowardsVelocity
  ;[1 1 1] Launch arrow and rotate towards velocity
  (Transformation|SetWorldRotation (Variables|Default|GetScene) (Math|Conversions|RotationFromXVector (Transformation|GetComponentVelocity (Variables|Default|GetCollision))) false false))

(event Custom|Blinking
  ;[1 1 1] Blink in and out before disappearing
  (Components|Timeline|SetPlayRate (Variables|Colors|GetOpacity) 1.75)
  (bind _opacityvalue (Timeline|opacity PlayFromStart)
    (:Update
      (Rendering|Material|SetScalarParameterValue (Variables|Default|GetdynamicMaterial) "opacity" _opacityvalue :!class /Script/Engine.MaterialInstanceDynamic))))

(event EventBeginPlay
  ;[1 1 1] Launch arrow and rotate towards velocity
  (bind _returnvalue (Rendering|Material|CreateDynamicMaterialInstance "/Game/Materials/Arrow_Dynamic_Inst.Arrow_Dynamic_Inst" :!class /Script/Engine.KismetMaterialLibrary))
  (bind _output_get (Variables|Default|SetdynamicMaterial _returnvalue))
  (Rendering|Material|SetMaterial (Variables|Default|GetArrow) 0 _output_get)
  (Physics|AddImpulse (Variables|Default|GetCollision) "0.000000,0.000000,300.000000" "None" true)
  (Utilities|Time|SetTimerbyFunctionName 0 "RotateTowardsVelocity" (Utilities|Time|GetWorldDeltaSeconds) true))

(fn ConstructionScript)