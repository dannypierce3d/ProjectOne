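; Bomb explosion actor that shakes the camera, scales its Explosion component along a timeline, then removes it and later itself.
; Overlapping a non-invincible character triggers invincibility, knocks the player backwards if holding the bomb or horizontally away otherwise, and briefly pauses movement.
; Damage and screen-change blocking run inside a loop over overlapped BP_NewScreen_01 actors.
; Other actors tagged "bombwilldestroy" receive a destroy message through the damage interface.
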(event OnComponentBeginOverlap(Explosion)
  (params (OverlappedComponent :type Primitive%20Component%20Object%20Reference) (OtherActor :type Actor%20Object%20Reference) (OtherComp :type Primitive%20Component%20Object%20Reference) (OtherBodyIndex :type Integer) (bFromSweep :type Boolean) (SweepResult :type Hit%20Result%20Structure%20%28by%20ref%29))
  (bind _returnvalue (Game|GetPlayerCharacter 0))
  (bind _returnvalue_2 (Game|GetPlayerCharacter 0))
  (bind _knockbackforce (Variables|Default|GetknockbackForce))
  (bind _returnvalue_3 (Transformation|GetActorForwardVector _returnvalue_2))
  (bind _returnvalue_4 (* _returnvalue_3 _knockbackforce))
  (bind _returnvalue_5 (* _returnvalue_4 -1.0))
  ;[1 1 1] Find objects caught in explosion and act on them accordingly
  (bind _asbp_character (Utilities|Casting|CastToBP_Character OtherActor)
    (:then
      (if (not (Variables|/Game/Blueprints/PlayerCharacter/BP_Character.BP_Character_C|GetisInvincible? _asbp_character))
        (Default|Invincible _asbp_character)
        (if (Utilities|TrueifHolding) ; Check if holding bomb
          ;;[1 1 1] If holding bomb, launch character backwards
          (Character|LaunchCharacter _returnvalue_2 (Math|Vector|MakeVector (.x _returnvalue_5) (.y _returnvalue_5) -3e+03) true true)
          (else
            ;;[1 1 1] Launch in direction opposite from explosion
            (bind (_launchvelocityx _launchvelocityy) (CallFunction|GetLaunchVelocity (Transformation|GetWorldLocation (Variables|/Script/Engine.Actor|GetRootComponent (Game|GetPlayerCharacter 0))) (Transformation|GetWorldLocation (Variables|Default|GetExplosion))))
            (Character|LaunchCharacter (Game|GetPlayerCharacter 0) (Math|Vector|MakeVector _launchvelocityx _launchvelocityy -3e+03) true true)))
        (bind _asbp_character_2 (Utilities|Casting|CastToBP_Character _returnvalue))
        (Default|PauseMovementforXSeconds _asbp_character_2 0.3)
        (for _array_element (Collision|GetOverlappingActors _returnvalue "/Game/Blueprints/BP_NewScreen_01.BP_NewScreen_01_C" :!class /Script/Engine.Actor) ; Don't allow screenchanging if still knocked back
          (bind _asbp_new_screen_01 (Utilities|Casting|CastToBP_NewScreen_01 _array_element))
          (Default|BlockKnockedBackPlayer _asbp_new_screen_01 0.5)
          (bind _asbp_character_3 (Utilities|Casting|CastToBP_Character _returnvalue))
          (Default|TakeDamage _asbp_character_3 0.5))))
    (:CastFailed
      (if (Actor|ActorHasTag OtherActor "bombwilldestroy")
        (if (Utilities|DoesObjectImplementInterface OtherActor "/Game/Blueprints/BP_damageInterface.BP_damageInterface_C")
          (Class|BPDamageInterface|DestroyObject(Message) OtherActor))))))

(event EventBeginPlay
  ;[1 1 1] Explode, shake camera and destroy actor
  (Camera|PlayWorldCameraShake "/Game/Blueprints/Projectiles/Bomb/bombShake.bombShake_C" (Transformation|GetActorLocation) 0.0 1e+05)
  (bind _explosionsize (Timeline|ExplosionSize PlayFromStart)
    (:Update
      (Transformation|SetWorldScale3D (Variables|Default|GetExplosion) (Math|Vector|MakeVector _explosionsize _explosionsize _explosionsize)))
    (:Finished
      (Components|DestroyComponent (Variables|Default|GetExplosion))
      (Utilities|FlowControl|Delay 4.0)
      (Actor|DestroyActor))))

(fn ConstructionScript)

(fn GetLaunchVelocity
  (params (otherVector :type Vector) (explosionVector :type Vector))
  (bind _returnvalue (Math|Vector|GetUnitDirection(Vector) otherVector explosionVector))
  (bind _knockbackforce (Variables|Default|GetknockbackForce))
  (bind _returnvalue_2 (Math|Vector|MakeVector (.x _returnvalue) (.y _returnvalue) 0.0))
  (bind _returnvalue_3 (Math|Vector|Normalize _returnvalue_2))
  (bind _returnvalue_4 (* (Math|Vector|MakeVector (.x _returnvalue_3) (.y _returnvalue_3) 0.0) -1.0))
  (bind _returnvalue_5 (* _returnvalue_4 _knockbackforce))
  ;[1 1 1] Compare vectors of explosion and other object to get launch velocity
  (return (.x _returnvalue_5) (.y _returnvalue_5)))