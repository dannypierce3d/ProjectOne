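; BP_Bomb_01 is a physics bomb projectile that explodes after a timed fuse or shortly after DestroyObject is called.
; If the fuse is lit at BeginPlay, a timeline pulses the mesh's scale and dynamic material flash parameter during the countdown.
; Both triggers share one path that removes components, spawns BP_BombExplosion_01 and destroys the actor.
; Tick adds downward acceleration while the capsule simulates physics, speeding its fall.
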(event Custom|StartBombFlash
  ;[1 1 1] Makes bomb flash and pulsate
  (bind _newtrack_0 (Timeline|bombFlash PlayFromStart)
    (:Update
      (Rendering|Material|SetScalarParameterValue (Variables|Default|GetdynamicMaterial) "bombFlash" _newtrack_0 :!class /Script/Engine.MaterialInstanceDynamic)
      (Transformation|SetWorldScale3D (Variables|Default|GetBomb) (+ (Variables|Default|GetbombScale) (/ _newtrack_0 2.0))))))

(event EventTick
  (params (DeltaSeconds :type Float%20%28single-precision%29))
  (bind _capsule (Variables|Default|GetCapsule))
  ;[1 1 1] Fall speed
  (if (Physics|IsSimulatingPhysics _capsule "None")
    (Physics|AddForce _capsule (Math|Vector|MakeVector 0.0 0.0 -5e+03) "None" true)))

(event EventBeginPlay
  ;[1 1 1] Apply dynamic material and start bomb timer
  (Variables|Default|SetbombScale (Transformation|GetWorldScale (Variables|Default|GetBomb)))
  (bind _returnvalue (Rendering|Material|CreateDynamicMaterialInstance "/Game/Materials/Bomb_Dynamic_Inst.Bomb_Dynamic_Inst" :!class /Script/Engine.KismetMaterialLibrary))
  (bind _output_get (Variables|Default|SetdynamicMaterial _returnvalue))
  (Rendering|Material|SetMaterial (Variables|Default|GetBomb) 0 _output_get)
  (if (Variables|Default|GetisFuseLit?)
    (CallFunction|StartBombFlash)
    (Utilities|FlowControl|Delay 4.0)
    (bind _output_get_2 (Variables|Default|SetexplosionLocation (Transformation|GetActorLocation)))
    (Components|DestroyComponent (Variables|Default|GetBomb))
    (Game|SpawnActorfromClass "/Game/Blueprints/Projectiles/Bomb/BP_BombExplosion_01.BP_BombExplosion_01_C" (Math|Transform|MakeTransform _output_get_2 "0, 0, 0" "1,1,1") "AlwaysSpawn" 0 0)
    (Actor|DestroyActor)))

(event EventDestroyObject
  ;[1 1 1] Apply dynamic material and start bomb timer
  (Utilities|FlowControl|Delay 0.15)
  (bind _output_get (Variables|Default|SetexplosionLocation (Transformation|GetActorLocation)))
  (Components|DestroyComponent (Variables|Default|GetBomb))
  (Game|SpawnActorfromClass "/Game/Blueprints/Projectiles/Bomb/BP_BombExplosion_01.BP_BombExplosion_01_C" (Math|Transform|MakeTransform _output_get "0, 0, 0" "1,1,1") "AlwaysSpawn" 0 0)
  (Actor|DestroyActor))

(fn ConstructionScript)