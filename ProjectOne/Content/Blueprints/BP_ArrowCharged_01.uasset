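; BP_ArrowCharged_01 is an arrow projectile that reacts to overlaps with tagged actors and cleans itself up.
; On "arrowstick" actors it drops its projectile movement to stick, then blinks via a looping visibility timer before destroying itself.
; On "arrowwilldestroy" actors only non-charged shots destroy themselves after a short delay.
; Ending overlap with an "arrowdestroy" component, intended as the screen boundary, disables collision and destroys the arrow.
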(event OnComponentEndOverlap(Collision)
  (params (OverlappedComponent :type Primitive%20Component%20Object%20Reference) (OtherActor :type Actor%20Object%20Reference) (OtherComp :type Primitive%20Component%20Object%20Reference) (OtherBodyIndex :type Integer))
  ;[1 1 1] Destroy arrow if it leaves screen
  (if (Components|ComponentHasTag OtherComp "arrowdestroy")
    (Collision|SetCollisionEnabled (Variables|Default|GetCollision) "NoCollision")
    (Actor|DestroyActor)))

(event OnComponentBeginOverlap(Collision)
  (params (OverlappedComponent :type Primitive%20Component%20Object%20Reference) (OtherActor :type Actor%20Object%20Reference) (OtherComp :type Primitive%20Component%20Object%20Reference) (OtherBodyIndex :type Integer) (bFromSweep :type Boolean) (SweepResult :type Hit%20Result%20Structure%20%28by%20ref%29))
  ;[1 1 1] Find if arrow should destroy object or get stuck in object
  (if (Actor|ActorHasTag OtherActor "arrowstick")
    (Components|DestroyComponent (Variables|Default|GetProjectileMovement))
    (Utilities|FlowControl|Delay 0.5)
    (Utilities|Time|SetTimerbyFunctionName 0 "Blinking" 0.0005 true)
    (Utilities|FlowControl|Delay 0.5)
    (Actor|DestroyActor)
    (elif (Actor|ActorHasTag OtherActor "arrowwilldestroy")
      (if (not (Variables|Default|GetisChargedShot?))
        (Utilities|FlowControl|Delay 0.05)
        (Actor|DestroyActor)))))

(event Custom|Blinking
  ;[1 1 1] Blink in and out before disappearing
  (Rendering|ToggleVisibility (Variables|Default|GetArrow) false))

(fn ConstructionScript)