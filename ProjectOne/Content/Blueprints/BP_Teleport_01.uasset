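; Screen-transition teleporter that moves the player to TeleportTo and switches the view to NewCamera when their capsule enters the trigger.
; A white fade hides the move while BP_GameInstance flags lock jumping, attacking and movement and block re-triggering.
; A looping timer then force-walks the character along the UpOrDown/LeftOrRight direction during fade-in.
; UpdateOldRotation stores the resulting yaw as one of four compass directions in the GameInstance before controls unlock.
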(event OnComponentBeginOverlap(TriggerVolume)
  (params (OverlappedComponent :type Primitive%20Component%20Object%20Reference) (OtherActor :type Actor%20Object%20Reference) (OtherComp :type Primitive%20Component%20Object%20Reference) (OtherBodyIndex :type Integer) (bFromSweep :type Boolean) (SweepResult :type Hit%20Result%20Structure%20%28by%20ref%29))
  (bind _teleportto (Variables|Default|GetteleportTo))
  (bind _returnvalue (Transformation|GetActorLocation _teleportto))
  (bind (_x _y _z) (Math|Vector|BreakVector _returnvalue))
  ;[1 1 1] Teleport
  (bind _asbp_character (Utilities|Casting|CastToBP_Character (Game|GetPlayerCharacter 0)))
  (if (== (Variables|/Script/Engine.Character|GetCapsuleComponent _asbp_character) OtherComp)
    (bind _asbp_game_instance (Utilities|Casting|CastToBP_GameInstance (Game|GetGameInstance)))
    (if (not (Variables|/Game/Blueprints/BP_GameInstance.BP_GameInstance_C|GetisTeleporting? _asbp_game_instance))
      (CameraFades|StartCameraFade (Game|GetPlayerCameraManager 0) 0.0 1.0 0.35 "(R=1.000000,G=1.000000,B=1.000000,A=1.000000)" false false)
      (bind _asbp_game_instance_2 (Utilities|Casting|CastToBP_GameInstance (Game|GetGameInstance)))
      (Variables|/Game/Blueprints/BP_GameInstance.BP_GameInstance_C|SetisTeleporting? _asbp_game_instance_2 true)
      (bind _asbp_game_instance_3 (Utilities|Casting|CastToBP_GameInstance (Game|GetGameInstance)))
      (Variables|/Game/Blueprints/BP_GameInstance.BP_GameInstance_C|SetallowJumping? _asbp_game_instance_3 false)
      (bind _asbp_game_instance_4 (Utilities|Casting|CastToBP_GameInstance (Game|GetGameInstance)))
      (Variables|/Game/Blueprints/BP_GameInstance.BP_GameInstance_C|SetallowAttacking? _asbp_game_instance_4 false)
      (bind _asbp_game_instance_5 (Utilities|Casting|CastToBP_GameInstance (Game|GetGameInstance)))
      (Variables|/Game/Blueprints/BP_GameInstance.BP_GameInstance_C|SetallowMovement? _asbp_game_instance_5 false)
      (bind _asbp_game_instance_6 (Utilities|Casting|CastToBP_GameInstance (Game|GetGameInstance)))
      (Variables|/Game/Blueprints/BP_GameInstance.BP_GameInstance_C|SetisBlocking? _asbp_game_instance_6 false)
      (Utilities|FlowControl|Delay 0.35) ; Delay for fade
      (Game|Player|SetViewTargetwithBlend (Game|GetPlayerController 0) (Variables|Default|GetnewCamera) 0.0 "VTBlend_EaseIn" 0.0 true) ; Change to new screen
      ;;[1 1 1] Disable Charge Attacks
      (bind _asbp_character_2 (Utilities|Casting|CastToBP_Character (Game|GetPlayerCharacter 0)))
      (Variables|/Game/Blueprints/PlayerCharacter/BP_Character.BP_Character_C|SetisCharging? _asbp_character_2 false)
      (Transformation|Teleport (Game|Player|GetPlayerPawn 0) (Math|Vector|MakeVector (+ _x 0.0) _y _z) (Math|Conversions|RotationFromXVector (Math|Vector|MakeVector (Variables|Default|GetupOrDown) (Variables|Default|GetleftOrRight) 0.0)))
      (CameraFades|StartCameraFade (Game|GetPlayerCameraManager 0) 1.0 0.0 0.35 "(R=1.000000,G=1.000000,B=1.000000,A=1.000000)" false false) ; End fade
      (Utilities|Time|SetTimerbyFunctionName 0 "Walk Forward" 0.0001 true)
      (Utilities|FlowControl|RetriggerableDelay 0.35)
      (CallFunction|UpdateOldRotation)
      (Utilities|Time|ClearTimerbyFunctionName 0 "Walk Forward")
      (bind _asbp_game_instance_7 (Utilities|Casting|CastToBP_GameInstance (Game|GetGameInstance)))
      (Variables|/Game/Blueprints/BP_GameInstance.BP_GameInstance_C|SetallowMovement? _asbp_game_instance_7 true)
      (bind _asbp_game_instance_8 (Utilities|Casting|CastToBP_GameInstance (Game|GetGameInstance)))
      (Variables|/Game/Blueprints/BP_GameInstance.BP_GameInstance_C|SetallowMovement? _asbp_game_instance_8 true)
      (bind _asbp_game_instance_9 (Utilities|Casting|CastToBP_GameInstance (Game|GetGameInstance)))
      (Variables|/Game/Blueprints/BP_GameInstance.BP_GameInstance_C|SetallowJumping? _asbp_game_instance_9 true)
      (bind _asbp_game_instance_10 (Utilities|Casting|CastToBP_GameInstance (Game|GetGameInstance)))
      (Variables|/Game/Blueprints/BP_GameInstance.BP_GameInstance_C|SetallowAttacking? _asbp_game_instance_10 true)
      (bind _asbp_game_instance_11 (Utilities|Casting|CastToBP_GameInstance (Game|GetGameInstance)))
      (Variables|/Game/Blueprints/BP_GameInstance.BP_GameInstance_C|SetisTeleporting? _asbp_game_instance_11 false))))

(event Custom|Walk%20Forward
  ;[1 1 1] Walk Up
  (Variables|/Script/Engine.CharacterMovementComponent|SetMaxWalkSpeed (Variables|/Script/Engine.Character|GetCharacterMovement (Game|GetPlayerCharacter 0)) 6e+02)
  (Pawn|Input|AddMovementInput (Game|GetPlayerCharacter 0) (Math|Vector|MakeVector (Variables|Default|GetupOrDown) (Variables|Default|GetleftOrRight) 0.0) 1.0 true))

(fn ConstructionScript)

(fn UpdateOldRotation
  (bind _returnvalue (Game|Player|GetPlayerPawn 0))
  (bind _returnvalue_2 (Transformation|GetActorRotation _returnvalue))
  (Variables|Default|SetcompassYaw (.yaw _returnvalue_2))
  (if (< (.yaw _returnvalue_2) 0.0)
    (bind _output_get (Variables|Default|SetcompassYaw (- 3.6e+02 (Math|Float|Absolute(Float) (Variables|Default|GetcompassYaw))))))
  (Utilities|FlowControl|Sequence
    (:then_0
      (if (or (Math|Float|InRange(Float) (Variables|Default|GetcompassYaw) 315.0 3.6e+02) (Math|Float|InRange(Float) (Variables|Default|GetcompassYaw) 0.0 45.0))
        (Development|PrintString "Up" false false)
        (bind _asbp_game_instance (Utilities|Casting|CastToBP_GameInstance (Game|GetGameInstance)))
        (Variables|/Game/Blueprints/BP_GameInstance.BP_GameInstance_C|SetoldRotation _asbp_game_instance 1.0)
        (Development|PrintString (Utilities|String|ToString(Float) _output_get) false false "(R=0.013877,G=0.033128,B=1.000000,A=1.000000)" :!label _label)))
    (:then_1
      (if (Math|Float|InRange(Float) (Variables|Default|GetcompassYaw) 45.0 135.0 false false)
        (Development|PrintString "Right" false false)
        (bind _asbp_game_instance_2 (Utilities|Casting|CastToBP_GameInstance (Game|GetGameInstance)))
        (Variables|/Game/Blueprints/BP_GameInstance.BP_GameInstance_C|SetoldRotation _asbp_game_instance_2 2.0)
        (goto _label)))
    (:then_2
      (if (Math|Float|InRange(Float) (Variables|Default|GetcompassYaw) 135.0 225.0)
        (Development|PrintString "Down" false false)
        (bind _asbp_game_instance_3 (Utilities|Casting|CastToBP_GameInstance (Game|GetGameInstance)))
        (Variables|/Game/Blueprints/BP_GameInstance.BP_GameInstance_C|SetoldRotation _asbp_game_instance_3 3.0)
        (goto _label)))
    (:then_3
      (if (Math|Float|InRange(Float) (Variables|Default|GetcompassYaw) 225.0 315.0 false false)
        (Development|PrintString "Left" false false)
        (bind _asbp_game_instance_4 (Utilities|Casting|CastToBP_GameInstance (Game|GetGameInstance)))
        (Variables|/Game/Blueprints/BP_GameInstance.BP_GameInstance_C|SetoldRotation _asbp_game_instance_4 4.0)
        (goto _label)))))