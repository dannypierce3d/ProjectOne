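; A ruby pickup that adds its value to the player's ruby count, capped at 999, and refreshes the HUD.
; On spawn it briefly ignores pickup channels, then, if set to fade, blinks via an opacity timeline and destroys itself unless collected.
; Overlap by the player's capsule or sword collects it, stops blinking and floats it above the player's head on a timeline before destroying it.
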(event OnComponentBeginOverlap(Box)
  (params (OverlappedComponent :type Primitive%20Component%20Object%20Reference) (OtherActor :type Actor%20Object%20Reference) (OtherComp :type Primitive%20Component%20Object%20Reference) (OtherBodyIndex :type Integer) (bFromSweep :type Boolean) (SweepResult :type Hit%20Result%20Structure%20%28by%20ref%29))
  ;[1 1 1] Pick up object
  (bind _asbp_character (Utilities|Casting|CastToBP_Character (Game|GetPlayerCharacter 0)))
  (if (== (Variables|/Script/Engine.Character|GetCapsuleComponent _asbp_character) OtherComp)
    (Variables|Default|SetisPickedUp true :!label _label)
    (Audio|Components|Audio|Stop (Variables|Colors|GetOpacity))
    (Rendering|Material|SetScalarParameterValue (Variables|Default|GetdynamicMaterial) "opacity" 1.0 :!class /Script/Engine.MaterialInstanceDynamic)
    (Rendering|SetActorHiddenInGame false)
    (Utilities|FlowControl|Delay 0.1)
    (CallFunction|AppearAbove) ; Make object appear above characters head
    ;;[1 1 1] Increase ruby count
    (bind _asbp_game_instance (Utilities|Casting|CastToBP_GameInstance (Game|GetGameInstance)))
    (Variables|/Game/Blueprints/BP_GameInstance.BP_GameInstance_C|SetplayerRubyCountFinal _asbp_game_instance (Math|Integer|Clamp(Integer) (+ (Variables|/Game/Blueprints/BP_GameInstance.BP_GameInstance_C|GetplayerRubyCountFinal _asbp_game_instance) (Variables|Default|GetrubyValue)) 0 999))
    (bind _asbp_character_2 (Utilities|Casting|CastToBP_Character (Game|GetPlayerCharacter 0)))
    (Default|UpdateRubyCount (Variables|/Game/Blueprints/PlayerCharacter/BP_Character.BP_Character_C|GetitemsHUDref _asbp_character_2))
    (else
      (bind _asbp_character_3 (Utilities|Casting|CastToBP_Character (Game|GetPlayerCharacter 0)))
      (if (== OtherComp (Variables|/Game/Blueprints/PlayerCharacter/BP_Character.BP_Character_C|GetSwordTest_01 _asbp_character_3))
        (goto _label)))))

(event Custom|AppearAbove
  (bind _returnvalue (Game|GetPlayerCharacter 0))
  (bind _returnvalue_2 (Transformation|GetActorLocation _returnvalue))
  ;[1 1 1] Appear above player after obtained
  (Components|DestroyComponent (Variables|Default|GetDecal))
  (Collision|SetActorEnableCollision false)
  (Physics|SetSimulatePhysics (Variables|Default|GetBox) false)
  (Game|Components|ProjectileMovement|StopSimulating (Variables|Default|GetProjectileMovement) (Collision|MakeHitResult false false 0.0 0.0 "0, 0, 0" "0, 0, 0" "0,0,1" "0,0,1" 0 0))
  (if true
    (bind _newtrack_0 (Timeline|AboveHeadAnimation Play)
      (:Update
        (Transformation|SetWorldLocation (Variables|Default|GetBox) (Math|Vector|MakeVector (.x _returnvalue_2) (.y _returnvalue_2) (+ (.z _returnvalue_2) _newtrack_0)) false false))
      (:Finished
        (Actor|DestroyActor)))))

(event Custom|Blinking
  ;[1 1 1] Make object visibility blink on and off
  (Components|Timeline|SetPlayRate (Variables|Colors|GetOpacity) 1.75)
  (bind _opacityvalue (Timeline|opacity PlayFromStart)
    (:Update
      (Rendering|Material|SetScalarParameterValue (Variables|Default|GetdynamicMaterial) "opacity" _opacityvalue :!class /Script/Engine.MaterialInstanceDynamic))))

(event EventBeginPlay
  (bind _ruby (Variables|Default|GetRuby))
  ;[1 1 1] Make unobtainable for a moment, then start counter till object disappears
  (bind _returnvalue (Rendering|Material|CreateDynamicMaterialInstance "/Game/Materials/Ruby_01_Dynamic_Inst.Ruby_01_Dynamic_Inst" :!class /Script/Engine.KismetMaterialLibrary))
  (bind _output_get (Variables|Default|SetdynamicMaterial _returnvalue))
  (Rendering|Material|SetMaterial (Variables|Default|GetRuby) 0 _output_get)
  (Collision|SetCollisionResponsetoChannel _ruby "ECC_GameTraceChannel2" "ECR_Ignore")
  (Collision|SetCollisionResponsetoChannel _ruby "ECC_GameTraceChannel3" "ECR_Ignore")
  (Utilities|FlowControl|Delay 0.5)
  (Collision|SetCollisionResponsetoChannel _ruby "ECC_GameTraceChannel2" "ECR_Overlap")
  (Collision|SetCollisionResponsetoChannel _ruby "ECC_GameTraceChannel3" "ECR_Overlap")
  (if (Variables|Default|GetshouldFade)
    (Utilities|FlowControl|Delay 7.0)
    (CallFunction|Blinking)
    (Utilities|FlowControl|Delay 2.0)
    (if (not (Variables|Default|GetisPickedUp))
      (Actor|DestroyActor))))

(fn ConstructionScript)