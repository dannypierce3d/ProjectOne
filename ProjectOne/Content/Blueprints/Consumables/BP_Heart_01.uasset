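; BP_Heart_01 is a heart pickup that restores one point of player health, capped at the maximum.
; On spawn it briefly ignores two custom trace channels on the heart so it cannot be collected immediately.
; Overlap of its box by the player's capsule or sword triggers collection, which stops physics, collision and projectile movement.
; A timeline then holds the heart above the player's head before destroying the actor.
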(event OnComponentBeginOverlap(Box)
  (params (OverlappedComponent :type Primitive%20Component%20Object%20Reference) (OtherActor :type Actor%20Object%20Reference) (OtherComp :type Primitive%20Component%20Object%20Reference) (OtherBodyIndex :type Integer) (bFromSweep :type Boolean) (SweepResult :type Hit%20Result%20Structure%20%28by%20ref%29))
  ;[1 1 1] Collect heart
  (bind _asbp_character (Utilities|Casting|CastToBP_Character (Game|GetPlayerCharacter 0)))
  (if (== (Variables|/Script/Engine.Character|GetCapsuleComponent _asbp_character) OtherComp)
    (Rendering|SetActorHiddenInGame false :!label _label)
    (Utilities|FlowControl|Delay 0.1)
    (CallFunction|AppearAbove)
    (bind _asbp_character_2 (Utilities|Casting|CastToBP_Character (Game|GetPlayerCharacter 0)))
    (Variables|/Game/Blueprints/PlayerCharacter/BP_Character.BP_Character_C|Sethealth _asbp_character_2 (Math|Float|Clamp(Float) (+ (Variables|/Game/Blueprints/PlayerCharacter/BP_Character.BP_Character_C|Gethealth _asbp_character_2) 1.0) 0.0 (Variables|/Game/Blueprints/PlayerCharacter/BP_Character.BP_Character_C|GetmaxHealth _asbp_character_2)))
    (else
      (bind _asbp_character_3 (Utilities|Casting|CastToBP_Character (Game|GetPlayerCharacter 0)))
      (if (== OtherComp (Variables|/Game/Blueprints/PlayerCharacter/BP_Character.BP_Character_C|GetSwordTest_01 _asbp_character_3))
        (goto _label)))))

(event Custom|AppearAbove
  (bind _returnvalue (Game|GetPlayerCharacter 0))
  (bind _returnvalue_2 (Transformation|GetActorLocation _returnvalue))
  ;[1 1 1] Make heart appear over head of character
  (Components|DestroyComponent (Variables|Default|GetDecal))
  (Collision|SetActorEnableCollision false)
  (Physics|SetSimulatePhysics (Variables|Default|GetHeart) false)
  (Game|Components|ProjectileMovement|StopSimulating (Variables|Default|GetProjectileMovement) (Collision|MakeHitResult false false 0.0 0.0 "0, 0, 0" "0, 0, 0" "0,0,1" "0,0,1" 0 0))
  (if true
    (bind _newtrack_0 (Timeline|Timeline_0 Play)
      (:Update
        (Transformation|SetWorldLocation (Variables|Default|GetHeart) (Math|Vector|MakeVector (.x _returnvalue_2) (.y _returnvalue_2) (+ (.z _returnvalue_2) _newtrack_0)) false false))
      (:Finished
        (Actor|DestroyActor)))))

(event EventBeginPlay
  (bind _heart (Variables|Default|GetHeart))
  ;[1 1 1] Make unobtainable for a moment
  (Collision|SetCollisionResponsetoChannel _heart "ECC_GameTraceChannel2" "ECR_Ignore")
  (Collision|SetCollisionResponsetoChannel _heart "ECC_GameTraceChannel3" "ECR_Ignore")
  (Utilities|FlowControl|Delay 0.5)
  (Collision|SetCollisionResponsetoChannel _heart "ECC_GameTraceChannel2" "ECR_Overlap")
  (Collision|SetCollisionResponsetoChannel _heart "ECC_GameTraceChannel3" "ECR_Overlap"))

(fn ConstructionScript)