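; Inventory component that holds items in a fixed number of slots and toggles the inventory window on the player's HUD.
; BeginPlay sizes the slot array, and AddToInventory tops up a matching partial stack or fills the first empty slot, recursing on any overflow.
; AddToInventory always returns true, with no check for a full inventory.
; ToggleInventory creates or removes the centered HUD widget, switching between UI-only and game-only input.
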(event EventBeginPlay
  (CallFunction|PrepareInventory))

(fn ToggleInventory
  (Variables|Default|GetinventoryWindow
    (:then
      (Widget|RemovefromParent (Variables|Default|GetinventoryWindow))
      (Variables|Default|SetinventoryWindow 0)
      (Input|SetInputModeGameOnly (Game|GetPlayerController 0)))
    (:else
      (bind _returnvalue (UserInterface|CreateWidget "/Game/Blueprints/Inventory/InventoryUI/InventoryWindow.InventoryWindow_C" 0 self))
      (Variables|Default|SetinventoryWindow _returnvalue)
      (bind _asmy_player_controller (Utilities|Casting|CastToMyPlayerController (Game|GetPlayerController 0)))
      (bind _returnvalue_2 (Class|CanvasPanel|AddChildtoCanvas (Variables|/Game/Blueprints/Inventory/InventoryUI/HUD.HUD_C|GetHudCanvas (Variables|/Game/Blueprints/MyPlayerController.MyPlayerController_C|GethudWidget _asmy_player_controller)) (Variables|Default|GetinventoryWindow)))
      (Class|CanvasPanelSlot|SetAutoSize _returnvalue_2 true)
      (Class|CanvasPanelSlot|SetAlignment _returnvalue_2 "(X=0.500000,Y=0.500000)")
      (Class|CanvasPanelSlot|SetAnchors _returnvalue_2 (Utilities|Struct|MakeAnchors "(X=0.500000,Y=0.500000)" "(X=0.500000,Y=0.500000)"))
      (Class|CanvasPanelSlot|SetPosition _returnvalue_2 (Variables|Default|Getposition))
      (Input|SetInputModeUIOnly (Game|GetPlayerController 0) (Variables|Default|GetinventoryWindow) "LockAlways"))))

(fn AddtoInventory
  (params (contentsToAdd :type Slot%20Structure%20Structure))
  (if (.isstackable (.itemstructure contentsToAdd))
    (bind _stackindex (Utilities|HasPartialStack contentsToAdd)
      (:true
        (CallFunction|AddtoStack contentsToAdd _stackindex))
      (:false
        (CallFunction|CreateStack contentsToAdd :!label _label)))
    (else
      (goto _label)))
  (return true))

(fn PrepareInventory
  (Utilities|Array|Resize (Variables|Default|Getinventory) (Variables|Default|GetnumberOfSlots)))

(fn CreateStack
  (params (contentToAdd :type Slot%20Structure%20Structure))
  (bind _inventory (Variables|Default|Getinventory))
  (Utilities|Array|SetArrayElem _inventory (Utilities|Array|FindItem _inventory (Utilities|Struct|MakeSlotStructure "(Name_2_89EDB07B483F755BE6E9A192C565518A=NSLOCTEXT(\"[8F04D8BA452855B4C0B1BC89C28C79BC]\", \"CD7F9AF1463580BC11D17EA612F10116\", \"None\"),isStackable_5_D63AB9324C1E46F144D13E99DFF5BA1B=True,thumbnail_8_E3C51F944BEF7D47E3A369A26A542E16=None,description_11_D36AF62B4B9C98FE8720D283831B8EFE=NSLOCTEXT(\"[8F04D8BA452855B4C0B1BC89C28C79BC]\", \"04F5A5304E281D6DBD43C4BACA934F1A\", \"None\"),isConsumable_14_9E1C27E94DBC9E2915C83DB7A8D4FE2C=True,maxStack_17_079F28484DAD983117416FAE1DA5BD6C=4,durability_20_A628574C41E2D5852AFBD893078FD49F=0.000000,class_23_4959D1304AB26694D368AABE384273EC=None)")) contentToAdd))

(fn AddtoStack
  (params (slotStructure :type Slot%20Structure%20Structure) (slotIndex :type Integer))
  (bind _inventory (Variables|Default|Getinventory))
  (bind _inventory_2 (Variables|Default|Getinventory))
  (bind _maxstack (Utilities|Struct|BreakItemStructure (.itemstructure slotStructure)))
  (bind _output (Utilities|Array|Get(acopy) _inventory slotIndex))
  (bind _output_get (LocalVariables|SetcurrentQuantity (.quantity _output)))
  (if (> (+ _output_get (.quantity (Utilities|Struct|BreakSlotStructure slotStructure))) (.maxstack (.itemstructure _output))) ; Check to see if new stack is needed
    (Utilities|Array|SetArrayElem (Variables|Default|Getinventory) slotIndex (Utilities|Struct|MakeSlotStructure (.itemstructure slotStructure) _maxstack))
    (CallFunction|AddtoInventory (Utilities|Struct|MakeSlotStructure (.itemstructure slotStructure) (- (.quantity slotStructure) (- _maxstack (LocalVariables|GetcurrentQuantity)))))
    (else
      (Utilities|Array|SetArrayElem _inventory_2 slotIndex (Utilities|Struct|MakeSlotStructure (.itemstructure slotStructure) (+ (.quantity (Utilities|Array|Get(acopy) _inventory_2 slotIndex)) (.quantity slotStructure)))) ; Not greater than stack size, add to current stack
    ))
  (return))