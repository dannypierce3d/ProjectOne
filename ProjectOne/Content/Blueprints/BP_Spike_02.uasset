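; BP_Spike_02 is a spike hazard that damages and knocks back the player while its Box is overlapped.
; Any overlap, not filtered by actor, starts a loop that rechecks every 0.2 seconds until the overlap ends.
; When player 0's BP_Character is not invincible, the loop triggers Invincible, launches them against their horizontal velocity and sharply downward, then subtracts clamped Health.
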(event OnComponentBeginOverlap(Box)
  (params (OverlappedComponent :type Primitive%20Component%20Object%20Reference) (OtherActor :type Actor%20Object%20Reference) (OtherComp :type Primitive%20Component%20Object%20Reference) (OtherBodyIndex :type Integer) (bFromSweep :type Boolean) (SweepResult :type Hit%20Result%20Structure%20%28by%20ref%29))
  (Variables|Default|SetisOnSpikes true)
  (CallFunction|StandingonSpikes))

(event OnComponentEndOverlap(Box)
  (params (OverlappedComponent :type Primitive%20Component%20Object%20Reference) (OtherActor :type Actor%20Object%20Reference) (OtherComp :type Primitive%20Component%20Object%20Reference) (OtherBodyIndex :type Integer))
  (Variables|Default|SetisOnSpikes false))

(event Custom|StandingOnSpikes
  (bind _returnvalue (Game|GetPlayerCharacter 0))
  (if (Variables|Default|GetisOnSpikes) :!label _label
    (bind _asbp_character (Utilities|Casting|CastToBP_Character (Game|GetPlayerCharacter 0)))
    (if (Variables|/Game/Blueprints/BP_Character.BP_Character_C|GetisInvincible? _asbp_character)
      _
      (else
        (Default|Invincible _asbp_character)
        (Variables|/Game/Blueprints/BP_Character.BP_Character_C|SetisInvincible? _asbp_character true)
        (Character|LaunchCharacter _returnvalue (Math|Vector|MakeVector (.x (* (Transformation|GetVelocity _asbp_character) -2.0)) (.y (* (Transformation|GetVelocity _asbp_character) -2.0)) -3e+03) false true)
        (bind _asbp_character_2 (Utilities|Casting|CastToBP_Character _returnvalue))
        (Variables|/Game/Blueprints/BP_Character.BP_Character_C|Sethealth _asbp_character_2 (Math|Float|Clamp(Float) (- (Variables|/Game/Blueprints/BP_Character.BP_Character_C|Gethealth _asbp_character_2) 0.51) 0.0 (Variables|/Game/Blueprints/BP_Character.BP_Character_C|GetmaxHealth _asbp_character_2)))))
    (Utilities|FlowControl|Delay 0.2)
    (goto _label)))

(fn ConstructionScript)