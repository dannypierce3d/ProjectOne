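; Screen actor for flip-screen camera transitions: when the player enters its trigger, the view blends to it.
; GameInstance stores old and new camera XY and flags; Tick compares positions to auto-walk the player along the transition axis, suspending jump and attack, then restoring them after a delay.
; Tick also makes edge boxes block falling players and records facing quadrant during walks.
; Leaving the trigger destroys overlapping bushes and respawns them through spawners.
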(event OnComponentEndOverlap(TriggerVolume)
  (params (OverlappedComponent :type Primitive%20Component%20Object%20Reference) (OtherActor :type Actor%20Object%20Reference) (OtherComp :type Primitive%20Component%20Object%20Reference) (OtherBodyIndex :type Integer))
  ;[1 1 1] Destroy existing bushes on exit and create new ones
  (Utilities|Casting|CastToBP_Character OtherActor)
  (Utilities|FlowControl|Delay 0.5)
  (bind _output_get (Variables|Default|SetoverlappingBush (Collision|GetOverlappingActors (Variables|Default|GetTriggerVolume) "/Game/Blueprints/BP_Bush_01.BP_Bush_01_C" :!class /Script/Engine.PrimitiveComponent)))
  (for _array_element _output_get
    (Actor|DestroyActor _array_element))
  (bind _output_get_2 (Variables|Default|SetoverlappingBushSpawner (Collision|GetOverlappingActors (Variables|Default|GetTriggerVolume) "/Game/Blueprints/BP_BushSpawner_01.BP_BushSpawner_01_C" :!class /Script/Engine.PrimitiveComponent)))
  (for _array_element_2 _output_get_2
    (bind _asbp_bush_spawner_01 (Utilities|Casting|CastToBP_BushSpawner_01 _array_element_2))
    (Default|Respawn _asbp_bush_spawner_01)))

(event OnComponentEndOverlap(TriggerVolumeSmaller)
  (params (OverlappedComponent :type Primitive%20Component%20Object%20Reference) (OtherActor :type Actor%20Object%20Reference) (OtherComp :type Primitive%20Component%20Object%20Reference) (OtherBodyIndex :type Integer))
  ;[1 1 1] Gets Old Camera position once
  (Utilities|Casting|CastToBP_Character OtherActor)
  (CallFunction|UpdateCamOld))

(event OnComponentBeginOverlap(TriggerVolume)
  (params (OverlappedComponent :type Primitive%20Component%20Object%20Reference) (OtherActor :type Actor%20Object%20Reference) (OtherComp :type Primitive%20Component%20Object%20Reference) (OtherBodyIndex :type Integer) (bFromSweep :type Boolean) (SweepResult :type Hit%20Result%20Structure%20%28by%20ref%29))
  ;[1 1 1] Camera Transfer
  (Utilities|Casting|CastToBP_Character OtherActor)
  (Variables|Default|SetshouldChangeCamNewValue true)
  (CallFunction|UpdateCamNew)
  (bind _asbp_game_instance (Utilities|Casting|CastToBP_GameInstance (Game|GetGameInstance)))
  (Variables|/Game/Blueprints/BP_GameInstance.BP_GameInstance_C|SetshouldWalk? _asbp_game_instance true)
  (bind _asbp_game_instance_2 (Utilities|Casting|CastToBP_GameInstance (Game|GetGameInstance)))
  (Variables|/Game/Blueprints/BP_GameInstance.BP_GameInstance_C|SetallowJumping? _asbp_game_instance_2 false)
  (bind _asbp_game_instance_3 (Utilities|Casting|CastToBP_GameInstance (Game|GetGameInstance)))
  (Variables|/Game/Blueprints/BP_GameInstance.BP_GameInstance_C|SetallowAttacking? _asbp_game_instance_3 false)
  (Game|Player|SetViewTargetwithBlend (Game|GetPlayerController 0) self 0.6 "VTBlend_Cubic" 0.0 true))

(event OnComponentBeginOverlap(TriggerVolumeSmaller)
  (params (OverlappedComponent :type Primitive%20Component%20Object%20Reference) (OtherActor :type Actor%20Object%20Reference) (OtherComp :type Primitive%20Component%20Object%20Reference) (OtherBodyIndex :type Integer) (bFromSweep :type Boolean) (SweepResult :type Hit%20Result%20Structure%20%28by%20ref%29))
  ;[1 1 1] Camera Transfer
  (Utilities|Casting|CastToBP_Character OtherActor)
  (CallFunction|UpdateCamNew)
  (Game|Player|SetViewTargetwithBlend (Game|GetPlayerController 0) self 0.6 "VTBlend_Cubic" 0.0 true))

(event Custom|Should%20Walk
  ;[1 1 1] Camera Transfer
)

(event EventTick
  (params (DeltaSeconds :type Float%20%28single-precision%29))
  (bind _returnvalue (Game|GetPlayerCharacter 0))
  (bind _returnvalue_2 (Game|GetPlayerCharacter 0))
  (bind _charactermovement (Variables|/Script/Engine.Character|GetCharacterMovement _returnvalue_2))
  (bind _charactermovement_2 (Variables|/Script/Engine.Character|GetCharacterMovement _returnvalue))
  ;[1 1 1] Walk after changing screens
  (CallFunction|UpdateCamNew)
  (CallFunction|NoJumponScreenChange)
  (bind _shouldwalk_ (|ShouldWalk?))
  (if _shouldwalk_
    (bind _asbp_game_instance (Utilities|Casting|CastToBP_GameInstance (Game|GetGameInstance)))
    (Variables|/Game/Blueprints/BP_GameInstance.BP_GameInstance_C|SetallowAttacking? _asbp_game_instance false) ; Disable Attacking while changing screens.
    (Variables|/Game/Blueprints/BP_GameInstance.BP_GameInstance_C|SetisTransferingScreen? _asbp_game_instance true)
    (Input|SetIgnoreMoveInput (Game|GetPlayerController 0) false)
    (CallFunction|FindPlayerWalkDirection)
    (bind _asbp_game_instance_2 (Utilities|Casting|CastToBP_GameInstance (Game|GetGameInstance)))
    (if (Variables|/Game/Blueprints/BP_GameInstance.BP_GameInstance_C|GetisTeleporting? _asbp_game_instance_2)
      (bind _asbp_game_instance_3 (Utilities|Casting|CastToBP_GameInstance (Game|GetGameInstance)))
      (Variables|/Game/Blueprints/BP_GameInstance.BP_GameInstance_C|SetshouldWalk? _asbp_game_instance_3 false)
      (Variables|/Game/Blueprints/BP_GameInstance.BP_GameInstance_C|SetisTransferingScreen? _asbp_game_instance_3 false)
      (else
        (Variables|/Script/Engine.CharacterMovementComponent|SetMaxWalkSpeed (Variables|/Script/Engine.Character|GetCharacterMovement (Game|GetPlayerCharacter 0)) 2e+02)
        (Variables|/Script/Engine.CharacterMovementComponent|SetbOrientRotationToMovement _charactermovement true)
        (Pawn|Input|AddMovementInput (Game|GetPlayerCharacter 0) (Math|Vector|MakeVector (Variables|Default|GetcamPosX) (Variables|Default|GetcamPosY) 0.0) 1.0 false)
        (CallFunction|UpdateOldRotation)
        (Utilities|FlowControl|Delay 0.54)
        (Variables|/Script/Engine.CharacterMovementComponent|SetbOrientRotationToMovement _charactermovement false)
        (bind _asbp_game_instance_4 (Utilities|Casting|CastToBP_GameInstance (Game|GetGameInstance)))
        (Variables|/Game/Blueprints/BP_GameInstance.BP_GameInstance_C|SetshouldWalk? _asbp_game_instance_4 false)
        (Variables|/Game/Blueprints/BP_GameInstance.BP_GameInstance_C|SetisTransferingScreen? _asbp_game_instance_4 false)
        (Input|EnableInput (Game|GetPlayerCharacter 0) (Game|GetPlayerController 0))
        (CallFunction|UpdateCamOld)
        (bind _asbp_game_instance_5 (Utilities|Casting|CastToBP_GameInstance (Game|GetGameInstance)))
        (Variables|/Game/Blueprints/BP_GameInstance.BP_GameInstance_C|SetallowJumping? _asbp_game_instance_5 true)
        (bind _asbp_game_instance_6 (Utilities|Casting|CastToBP_GameInstance (Game|GetGameInstance)))
        (Variables|/Game/Blueprints/BP_GameInstance.BP_GameInstance_C|SetallowAttacking? _asbp_game_instance_6 true)
        (bind _asbp_game_instance_7 (Utilities|Casting|CastToBP_GameInstance (Game|GetGameInstance)))
        (if (Variables|/Game/Blueprints/BP_GameInstance.BP_GameInstance_C|GetisBlocking? _asbp_game_instance_7)
          (Variables|/Script/Engine.CharacterMovementComponent|SetMaxWalkSpeed _charactermovement_2 2e+02 :!label _label)
          (else
            (bind _asbp_character (Utilities|Casting|CastToBP_Character _returnvalue))
            (if (Variables|/Game/Blueprints/BP_Character.BP_Character_C|GetisCharging? _asbp_character)
              (goto _label)
              (else
                (Variables|/Script/Engine.CharacterMovementComponent|SetMaxWalkSpeed _charactermovement_2 6e+02)))))
        (bind _asbp_bush_spawner_01 (Utilities|Casting|CastToBP_BushSpawner_01 (Components|GetOwner)))
        (Default|Respawn _asbp_bush_spawner_01)))))

(fn ConstructionScript)

(fn NoJumponScreenChange
  ;[1 1 1] Doesn't allow player to jump while attempting to change screens
  (if (AI|Components|NavMovement|IsFalling (Variables|/Script/Engine.Character|GetCharacterMovement (Game|GetPlayerCharacter 0)))
    (Collision|SetCollisionResponsetoChannel (Variables|Default|GetCollisionBox_Left_01) "ECC_Pawn" "ECR_Block")
    (else
      (Collision|SetCollisionResponsetoChannel (Variables|Default|GetCollisionBox_Left_01) "ECC_Pawn" "ECR_Ignore")))
  (return))

(fn UpdateCamNew
  (bind _camera (Variables|Default|GetCamera))
  (bind _returnvalue (Transformation|GetWorldLocation _camera))
  ;[1 1 1] Updates the new camera values to be compared with old cam
  (if (Variables|Default|GetshouldChangeCamNewValue)
    (bind _asbp_game_instance (Utilities|Casting|CastToBP_GameInstance (Game|GetGameInstance)))
    (Variables|/Game/Blueprints/BP_GameInstance.BP_GameInstance_C|SetcamXNew _asbp_game_instance (.x _returnvalue))
    (Variables|/Game/Blueprints/BP_GameInstance.BP_GameInstance_C|SetcamYNew _asbp_game_instance (.y _returnvalue))
    (Variables|Default|SetshouldChangeCamNewValue false))
  (return))

(fn FindPlayerWalkDirection
  ;[1 1 1] Compare old and New camera locations to determine which direction to walk
  (bind _asbp_game_instance (Utilities|Casting|CastToBP_GameInstance (Game|GetGameInstance))
    (:then
      (if (== (Variables|/Game/Blueprints/BP_GameInstance.BP_GameInstance_C|GetcamX _asbp_game_instance) (Variables|/Game/Blueprints/BP_GameInstance.BP_GameInstance_C|GetcamXNew _asbp_game_instance))
        (if (> (Variables|/Game/Blueprints/BP_GameInstance.BP_GameInstance_C|GetcamY _asbp_game_instance) (Variables|/Game/Blueprints/BP_GameInstance.BP_GameInstance_C|GetcamYNew _asbp_game_instance))
          (Variables|Default|SetcamPosY -1.0)
          (Variables|Default|SetcamPosX 0.0)
          (else
            (Variables|Default|SetcamPosY 1.0)
            (Variables|Default|SetcamPosX 0.0)))
        (elif (== (Variables|/Game/Blueprints/BP_GameInstance.BP_GameInstance_C|GetcamY _asbp_game_instance) (Variables|/Game/Blueprints/BP_GameInstance.BP_GameInstance_C|GetcamYNew _asbp_game_instance))
          (if (> (Variables|/Game/Blueprints/BP_GameInstance.BP_GameInstance_C|GetcamX _asbp_game_instance) (Variables|/Game/Blueprints/BP_GameInstance.BP_GameInstance_C|GetcamXNew _asbp_game_instance))
            (Variables|Default|SetcamPosX -1.0)
            (Variables|Default|SetcamPosY 0.0)
            (else
              (Variables|Default|SetcamPosX 1.0)
              (Variables|Default|SetcamPosY 0.0))))))
    (:CastFailed
      _))
  (return))

(fn UpdateCamOld
  (bind _camera (Variables|Default|GetCamera))
  (bind _returnvalue (Transformation|GetWorldLocation _camera))
  ;[1 1 1] Grabs current cam value and places it in old
  (bind _asbp_game_instance (Utilities|Casting|CastToBP_GameInstance (Game|GetGameInstance))
    (:then
      (Variables|/Game/Blueprints/BP_GameInstance.BP_GameInstance_C|SetcamX _asbp_game_instance (.x _returnvalue))
      (Variables|/Game/Blueprints/BP_GameInstance.BP_GameInstance_C|SetcamY _asbp_game_instance (.y _returnvalue)))
    (:CastFailed
      _))
  (return))

(fn UpdateOldRotation
  (bind _returnvalue (Game|Player|GetPlayerPawn 0))
  (bind _returnvalue_2 (Transformation|GetActorRotation _returnvalue))
  (Variables|Default|SetcompassYaw (.yaw _returnvalue_2))
  (if (< (.yaw _returnvalue_2) 0.0)
    (bind _output_get (Variables|Default|SetcompassYaw (- 3.6e+02 (Math|Float|Absolute(Float) (Variables|Default|GetcompassYaw))))))
  (Utilities|FlowControl|Sequence
    (:then_0
      (if (or (Math|Float|InRange(Float) (Variables|Default|GetcompassYaw) 315.0 3.6e+02) (Math|Float|InRange(Float) (Variables|Default|GetcompassYaw) 0.0 45.0))
        (Development|PrintString "Up" false false)
        (bind _asbp_game_instance (Utilities|Casting|CastToBP_GameInstance (Game|GetGameInstance)))
        (Variables|/Game/Blueprints/BP_GameInstance.BP_GameInstance_C|SetoldRotation _asbp_game_instance 1.0)
        (Development|PrintString (Utilities|String|ToString(Float) _output_get) false false "(R=0.013877,G=0.033128,B=1.000000,A=1.000000)" :!label _label)))
    (:then_1
      (if (Math|Float|InRange(Float) (Variables|Default|GetcompassYaw) 45.0 135.0 false false)
        (Development|PrintString "Right" false false)
        (bind _asbp_game_instance_2 (Utilities|Casting|CastToBP_GameInstance (Game|GetGameInstance)))
        (Variables|/Game/Blueprints/BP_GameInstance.BP_GameInstance_C|SetoldRotation _asbp_game_instance_2 2.0)
        (goto _label)))
    (:then_2
      (if (Math|Float|InRange(Float) (Variables|Default|GetcompassYaw) 135.0 225.0)
        (Development|PrintString "Down" false false)
        (bind _asbp_game_instance_3 (Utilities|Casting|CastToBP_GameInstance (Game|GetGameInstance)))
        (Variables|/Game/Blueprints/BP_GameInstance.BP_GameInstance_C|SetoldRotation _asbp_game_instance_3 3.0)
        (goto _label)))
    (:then_3
      (if (Math|Float|InRange(Float) (Variables|Default|GetcompassYaw) 225.0 315.0 false false)
        (Development|PrintString "Left" false false)
        (bind _asbp_game_instance_4 (Utilities|Casting|CastToBP_GameInstance (Game|GetGameInstance)))
        (Variables|/Game/Blueprints/BP_GameInstance.BP_GameInstance_C|SetoldRotation _asbp_game_instance_4 4.0)
        (goto _label)))))