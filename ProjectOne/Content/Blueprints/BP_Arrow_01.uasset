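; Bow arrow actor with projectile movement that attaches to the player character's bow on BeginPlay.
; Tick continually sets its location to the character's ArrowLaunchPoint and its rotation to the bow's, with yaw flipped.
; Collision overlaps are tag-driven: "arrowstick" removes projectile movement, blinks the mesh, then destroys it; "arrowwilldestroy" destroys uncharged shots after a brief delay.
; Ending overlap with an "arrowdestroy" component destroys it immediately.
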(event OnComponentEndOverlap(Collision)
  (params (OverlappedComponent :type Primitive%20Component%20Object%20Reference) (OtherActor :type Actor%20Object%20Reference) (OtherComp :type Primitive%20Component%20Object%20Reference) (OtherBodyIndex :type Integer))
  (if (Components|ComponentHasTag OtherComp "arrowdestroy")
    (Collision|SetCollisionEnabled (Variables|Default|GetCollision) "NoCollision")
    (Actor|DestroyActor)))

(event OnComponentBeginOverlap(Collision)
  (params (OverlappedComponent :type Primitive%20Component%20Object%20Reference) (OtherActor :type Actor%20Object%20Reference) (OtherComp :type Primitive%20Component%20Object%20Reference) (OtherBodyIndex :type Integer) (bFromSweep :type Boolean) (SweepResult :type Hit%20Result%20Structure%20%28by%20ref%29))
  (if (Actor|ActorHasTag OtherActor "arrowstick")
    (Components|DestroyComponent (Variables|Default|GetProjectileMovement))
    (Utilities|FlowControl|Delay 0.5)
    (Utilities|Time|SetTimerbyFunctionName 0 "Blinking" 0.0005 true)
    (Utilities|FlowControl|Delay 0.5)
    (Actor|DestroyActor)
    (elif (Actor|ActorHasTag OtherActor "arrowwilldestroy")
      (if (not (Variables|Default|GetisChargedShot?))
        (Utilities|FlowControl|Delay 0.05)
        (Actor|DestroyActor)))))

(event Custom|Blinking
  (Rendering|ToggleVisibility (Variables|Default|GetArrow) false))

(event EventBeginPlay
  (bind _asbp_character (Utilities|Casting|CastToBP_Character (Game|GetPlayerCharacter 0)))
  (Transformation|AttachComponentToComponent (Variables|/Game/Blueprints/BP_Character.BP_Character_C|GetBowTest_01 _asbp_character) "None" "SnapToTarget" "SnapToTarget" "KeepWorld" false))

(event EventTick
  (params (DeltaSeconds :type Float%20%28single-precision%29))
  (bind _asbp_character (Utilities|Casting|CastToBP_Character (Game|GetPlayerCharacter 0)))
  (Transformation|SetActorLocation (Transformation|GetWorldLocation (Variables|/Game/Blueprints/BP_Character.BP_Character_C|GetArrowLaunchPoint _asbp_character)) false false)
  (Transformation|SetActorRotation (Math|Rotator|MakeRotator (.roll (Transformation|GetWorldRotation (Variables|/Game/Blueprints/BP_Character.BP_Character_C|GetBowTest_01 _asbp_character))) (.pitch (Transformation|GetWorldRotation (Variables|/Game/Blueprints/BP_Character.BP_Character_C|GetBowTest_01 _asbp_character))) (+ (.yaw (Transformation|GetWorldRotation (Variables|/Game/Blueprints/BP_Character.BP_Character_C|GetBowTest_01 _asbp_character))) 1.8e+02))))

(fn ConstructionScript)