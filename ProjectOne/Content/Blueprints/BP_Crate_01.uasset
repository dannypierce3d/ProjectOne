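; BP_Crate_01 is a physics crate that the player can destroy with a sword.
; Every Tick applies a downward velocity-change impulse to the Crate component as added gravity.
; An overlap with the player character's SwordTest01 component while IsAttacking is true fires a DoOnce that waits briefly, hides the actor, disables its collision and destroys it.
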(event OnComponentBeginOverlap(Crate)
  (params (OverlappedComponent :type Primitive%20Component%20Object%20Reference) (OtherActor :type Actor%20Object%20Reference) (OtherComp :type Primitive%20Component%20Object%20Reference) (OtherBodyIndex :type Integer) (bFromSweep :type Boolean) (SweepResult :type Hit%20Result%20Structure%20%28by%20ref%29))
  ;[1 1 1] Destroy crate if hit with sword
  (bind _asbp_character (Utilities|Casting|CastToBP_Character (Game|GetPlayerCharacter 0)))
  (if (== (Variables|/Game/Blueprints/BP_Character.BP_Character_C|GetSwordTest_01 _asbp_character) OtherComp)
    (if (Variables|/Game/Blueprints/BP_Character.BP_Character_C|GetisAttacking? _asbp_character)
      (Utilities|FlowControl|DoOnce false
        (:Completed
          (Utilities|FlowControl|Delay 0.15)
          (Rendering|SetActorHiddenInGame true)
          (Collision|SetActorEnableCollision false)
          (Actor|DestroyActor))))))

(event EventTick
  (params (DeltaSeconds :type Float%20%28single-precision%29))
  ;[1 1 1] Add downward force
  (Physics|AddImpulse (Variables|Default|GetCrate) "0, 0,-40.000000" "None" true))

(fn ConstructionScript)