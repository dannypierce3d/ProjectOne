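; BP_Bush_01 is a destructible bush that drops a ruby when broken.
; It breaks when its Box hits anything but the player, or its Sphere overlaps an arrow or the player's attacking sword.
; While the Box simulates physics, Tick applies a downward impulse to quicken falls.
; DestroyBush runs once, hiding the bush, spawning BP_Ruby_02 after a brief delay, then destroying the actor; a velocity check remains unwired.
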(event OnComponentBeginOverlap(Sphere)
  (params (OverlappedComponent :type Primitive%20Component%20Object%20Reference) (OtherActor :type Actor%20Object%20Reference) (OtherComp :type Primitive%20Component%20Object%20Reference) (OtherBodyIndex :type Integer) (bFromSweep :type Boolean) (SweepResult :type Hit%20Result%20Structure%20%28by%20ref%29))
  ;[1 1 1] Destroy with sword only when attacking
  (bind _asbp_character (Utilities|Casting|CastToBP_Character (Game|GetPlayerCharacter 0)))
  (if (== (Variables|/Game/Blueprints/PlayerCharacter/BP_Character.BP_Character_C|GetSwordTest_01 _asbp_character) OtherComp)
    (if (Variables|/Game/Blueprints/PlayerCharacter/BP_Character.BP_Character_C|GetisAttacking? _asbp_character)
      (CallFunction|DestroyBush :!label _label))
    (elif (Actor|ActorHasTag OtherActor "arrow")
      (goto _label))))

(event OnComponentHit(Box)
  (params (HitComponent :type Primitive%20Component%20Object%20Reference) (OtherActor :type Actor%20Object%20Reference) (OtherComp :type Primitive%20Component%20Object%20Reference) (NormalImpulse :type Vector :default "0, 0, 0") (Hit :type Hit%20Result%20Structure%20%28by%20ref%29))
  ;[1 1 1] Destroy Bush when thrown/dropped
  (if (not (== (Game|GetPlayerCharacter 0) OtherActor))
    (Development|PrintString "HITFLOOR" false false "(R=0.000000,G=0.000000,B=0.000000,A=1.000000)")
    (CallFunction|DestroyBush)))

(event Custom|SpawnItem
  (bind _returnvalue (Transformation|GetActorTransform))
  ;[1 1 1] Spawn Item
  (Utilities|FlowControl|DoOnce false
    (:Completed
      (bind _returnvalue_2 (Game|SpawnActorfromClass "/Game/Blueprints/Consumables/BP_Ruby_02.BP_Ruby_02_C" (Transformation|GetActorTransform) "AlwaysSpawn" 0 0))
      (bind _output_get (Variables|Default|SetSpawn_Ruby _returnvalue_2))
      (Transformation|SetActorTransform _output_get (Math|Transform|MakeTransform (.location _returnvalue) (.rotation _returnvalue) "1,1,1")))))

(event Custom|DestroyBush
  ;[1 1 1] Destroy Bush
  (Utilities|FlowControl|DoOnce false
    (:Completed
      (Rendering|SetActorHiddenInGame true)
      (Utilities|FlowControl|Delay 0.1)
      (CallFunction|SpawnItem)
      (Actor|DestroyActor))))

(event EventTick
  (params (DeltaSeconds :type Float%20%28single-precision%29))
  ;[1 1 1] Fall speed
  (if (Physics|IsSimulatingPhysics (Variables|Default|GetBox) "None")
    (Physics|AddImpulse (Variables|Default|GetBox) "0, 0,-100.000000" "None" true)))

(fn ConstructionScript)