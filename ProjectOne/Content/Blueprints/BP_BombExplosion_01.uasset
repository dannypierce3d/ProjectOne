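; Bomb blast actor that scales its Explosion component over a timeline, removes it, then destroys itself after a delay.
; Overlapping a non-invincible BP_Character triggers invincibility, knocks player 0 back and briefly pauses their movement.
; Knockback opposes the player's facing if TrueIfHolding reports a held bomb, otherwise it uses FindLaunchDirection, mirrored in Y by side.
; Overlapped bushes tagged "bombwilldestroy" are destroyed.
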(event OnComponentBeginOverlap(Explosion)
  (params (OverlappedComponent :type Primitive%20Component%20Object%20Reference) (OtherActor :type Actor%20Object%20Reference) (OtherComp :type Primitive%20Component%20Object%20Reference) (OtherBodyIndex :type Integer) (bFromSweep :type Boolean) (SweepResult :type Hit%20Result%20Structure%20%28by%20ref%29))
  (bind _returnvalue (Game|GetPlayerCharacter 0))
  (bind (_xlaunchvalue _ylaunchvalue) (Utilities|FindLaunchDirection))
  (bind _knockbackforce (Variables|Default|GetknockbackForce))
  (bind _returnvalue_2 (Transformation|GetActorForwardVector _returnvalue))
  (bind _returnvalue_3 (* _returnvalue_2 _knockbackforce))
  (bind _returnvalue_4 (* _returnvalue_3 -1.0))
  ;[1 1 1] Find objects caught in explosion and act on them accordingly
  (bind _asbp_character (Utilities|Casting|CastToBP_Character OtherActor)
    (:then
      (if (not (Variables|/Game/Blueprints/BP_Character.BP_Character_C|GetisInvincible? _asbp_character))
        (Default|Invincible _asbp_character)
        (if (Utilities|TrueifHolding) ; Check if holding bomb
          ;;[1 1 1] Is holding bomb
          (Character|LaunchCharacter _returnvalue (Math|Vector|MakeVector (.x _returnvalue_4) (.y _returnvalue_4) -3e+03) true true)
          (else
            ;;[1 1 1] Check if stand to right or left of bomb
            (if (> (.y (Transformation|GetActorLocation (Game|GetPlayerCharacter 0))) (.y (Transformation|GetWorldLocation (Variables|Default|GetExplosion))))
              (Development|PrintString "to the right of bomb" false)
              (Character|LaunchCharacter (Game|GetPlayerCharacter 0) (Math|Vector|MakeVector _xlaunchvalue _ylaunchvalue -3e+03) true true)
              (else
                (Development|PrintString "to the left of bomb" false)
                (Character|LaunchCharacter (Game|GetPlayerCharacter 0) (Math|Vector|MakeVector _xlaunchvalue (* _ylaunchvalue -1.0) -3e+03) true true)))))
        (bind _asbp_character_2 (Utilities|Casting|CastToBP_Character (Game|GetPlayerCharacter 0)))
        (Default|PauseMovement _asbp_character_2 0.35)))
    (:CastFailed
      (if (Actor|ActorHasTag OtherActor "bombwilldestroy")
        (bind _asbp_bush_01 (Utilities|Casting|CastToBP_Bush_01 OtherActor))
        (Default|DestroyBush _asbp_bush_01)))))

(event EventBeginPlay
  ;[1 1 1] Explode and destroy actor
  (bind _explosionsize (Timeline|ExplosionSize PlayFromStart)
    (:Update
      (Transformation|SetWorldScale3D (Variables|Default|GetExplosion) (Math|Vector|MakeVector _explosionsize _explosionsize _explosionsize)))
    (:Finished
      (Components|DestroyComponent (Variables|Default|GetExplosion))
      (Utilities|FlowControl|Delay 4.0)
      (Actor|DestroyActor))))

(fn ConstructionScript)