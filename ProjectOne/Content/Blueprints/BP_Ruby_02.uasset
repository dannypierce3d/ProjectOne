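; Ruby pickup that adds 20 to the game instance's capped ruby count and refreshes the HUD.
; It ignores two trace channels briefly after spawning, then overlaps; with ShouldFade set, it later blinks via a looping timer and destroys itself.
; Overlap by the player's capsule or sword triggers AppearAbove, which disables collision and movement, then uses a timeline to float it over the player before destruction.
; Save-game code is present but never runs.
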(event OnComponentBeginOverlap(Box)
  (params (OverlappedComponent :type Primitive%20Component%20Object%20Reference) (OtherActor :type Actor%20Object%20Reference) (OtherComp :type Primitive%20Component%20Object%20Reference) (OtherBodyIndex :type Integer) (bFromSweep :type Boolean) (SweepResult :type Hit%20Result%20Structure%20%28by%20ref%29))
  (bind _asbp_character (Utilities|Casting|CastToBP_Character (Game|GetPlayerCharacter 0)))
  (if (== (Variables|/Script/Engine.Character|GetCapsuleComponent _asbp_character) OtherComp)
    (Rendering|SetActorHiddenInGame false :!label _label)
    (Utilities|FlowControl|Delay 0.1)
    (CallFunction|AppearAbove)
    (bind _asbp_game_instance (Utilities|Casting|CastToBP_GameInstance (Game|GetGameInstance)))
    (Variables|/Game/Blueprints/BP_GameInstance.BP_GameInstance_C|SetplayerRubyCountFinal _asbp_game_instance (Math|Integer|Clamp(Integer) (+ (Variables|/Game/Blueprints/BP_GameInstance.BP_GameInstance_C|GetplayerRubyCountFinal _asbp_game_instance) 20) 0 999))
    (bind _asbp_character_2 (Utilities|Casting|CastToBP_Character (Game|GetPlayerCharacter 0)))
    (Default|UpdateRubyCount (Variables|/Game/Blueprints/BP_Character.BP_Character_C|GetitemsHUDref _asbp_character_2))
    (else
      (bind _asbp_character_3 (Utilities|Casting|CastToBP_Character (Game|GetPlayerCharacter 0)))
      (if (== OtherComp (Variables|/Game/Blueprints/BP_Character.BP_Character_C|GetSwordTest_01 _asbp_character_3))
        (goto _label)))))

(event Custom|AppearAbove
  (bind _returnvalue (Game|GetPlayerCharacter 0))
  (bind _returnvalue_2 (Transformation|GetActorLocation _returnvalue))
  (Utilities|Time|ClearTimerbyFunctionName 0 "Blinking")
  (Rendering|SetVisibility (Variables|Default|GetBox) true false)
  (Components|DestroyComponent (Variables|Default|GetDecal))
  (Collision|SetActorEnableCollision false)
  (Physics|SetSimulatePhysics (Variables|Default|GetBox) false)
  (Game|Components|ProjectileMovement|StopSimulating (Variables|Default|GetProjectileMovement) (Collision|MakeHitResult false false 0.0 "0, 0, 0" "0, 0, 0" "0,0,1" "0,0,1" 0 0 0))
  (if true
    (bind _newtrack_0 (Timeline|Timeline_1 Play)
      (:Update
        (Transformation|SetWorldLocation (Variables|Default|GetBox) (Math|Vector|MakeVector (.x _returnvalue_2) (.y _returnvalue_2) (+ (.z _returnvalue_2) _newtrack_0)) false false))
      (:Finished
        (Actor|DestroyActor)))))

(event Custom|Blinking
  (Rendering|ToggleVisibility (Variables|Default|GetRuby) false))

(event EventBeginPlay
  (bind _ruby (Variables|Default|GetRuby))
  (Collision|SetCollisionResponsetoChannel _ruby "ECC_GameTraceChannel2" "ECR_Ignore")
  (Collision|SetCollisionResponsetoChannel _ruby "ECC_GameTraceChannel3" "ECR_Ignore")
  (Utilities|FlowControl|Delay 0.5)
  (Collision|SetCollisionResponsetoChannel _ruby "ECC_GameTraceChannel2" "ECR_Overlap")
  (Collision|SetCollisionResponsetoChannel _ruby "ECC_GameTraceChannel3" "ECR_Overlap")
  (if (Variables|Default|GetshouldFade)
    (Utilities|FlowControl|Delay 7.0)
    (Utilities|Time|SetTimerbyFunctionName 0 "Blinking" 0.0005 true)
    (Utilities|FlowControl|Delay 2.0)
    (Actor|DestroyActor)))

(fn ConstructionScript)