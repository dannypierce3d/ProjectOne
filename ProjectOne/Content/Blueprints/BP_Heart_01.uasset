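; BP_Heart_01 is a health pickup actor that restores one point of health to the player.
; On its first overlap, guarded by DoOnce, it casts player 0 to BP_Character_03 and raises Health, clamped to MaxHealth.
; It then hides itself and destroys the actor after a short delay.
; The overlapping actor is not checked, so any overlap triggers the heal.
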(event EventBeginPlay)

(event Collision|EventActorBeginOverlap
  (params (OtherActor :type Actor%20Object%20Reference))
  (Utilities|FlowControl|DoOnce false
    (:Completed
      (bind _asbp_character_03 (Utilities|Casting|CastToBP_Character_03 (Game|GetPlayerCharacter 0)))
      (Variables|/Game/Blueprints/BP_Character_03.BP_Character_03_C|Sethealth _asbp_character_03 (Math|Float|Clamp(Float) (+ (Variables|/Game/Blueprints/BP_Character_03.BP_Character_03_C|Gethealth _asbp_character_03) 1.0) 0.0 (Variables|/Game/Blueprints/BP_Character_03.BP_Character_03_C|GetmaxHealth _asbp_character_03)))
      (Rendering|SetActorHiddenInGame true)
      (Utilities|FlowControl|Delay 3.0)
      (Actor|DestroyActor))))

(event EventTick
  (params (DeltaSeconds :type Float%20%28single-precision%29)))

(fn ConstructionScript)